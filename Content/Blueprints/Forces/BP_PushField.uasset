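; BP_PushField is a Chaos physics field actor that pushes physics objects inside a sphere along an arrow's direction.
; Its Fire function applies a linear velocity field built from a uniform vector along the Arrow, multiplied by a non-fading radial falloff and scaled by ForceMagnitude.
; A culling field with a second radial falloff at the Sphere's radius and location limits the push to that volume.
; The event graph holds no logic.
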(event EventBeginPlay)

(event Collision|EventActorBeginOverlap
  (params (OtherActor :type Actor%20Object%20Reference)))

(event EventTick
  (params (DeltaSeconds :type Float%20%28single-precision%29)))

(fn ConstructionScript)

(fn Fire
  (bind _sphere (Variables|Default|GetSphere))
  (bind _returnvalue (Transformation|GetWorldLocation _sphere))
  (bind _sphereradius (Variables|/Script/Engine.SphereComponent|GetSphereRadius _sphere))
  (Class|FieldSystemComponent|ApplyPhysicsField (Variables|Default|GetFieldSystem) true "Field_LinearVelocity" 0 (Field|SetCullingField (Variables|Default|GetCullingField) (Field|SetRadialFalloff (Variables|Default|GetRadialFalloff1) 1.0 0.0 1.0 0.0 _sphereradius _returnvalue "Field_FallOff_None") (Field|SetOperatorField (Variables|Default|GetOperatorField) (Variables|Default|GetForceMagnitude) (Field|SetRadialFalloff (Variables|Default|GetRadialFalloff) 1.0 0.0 1.0 0.0 _sphereradius _returnvalue "Field_FallOff_None") (Field|SetUniformVector (Variables|Default|GetUniformVector) 1.0 (Math|Vector|GetForwardVector (Variables|Default|GetArrow))) "Field_Multiply") "Field_Culling_Outside")))